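; BP_DataActor spawns and removes location probe actors by point type, using geographic rows from a data table.
; Spawning converts latitude/longitude through GeoReferencing, creates tall scaled BP_CustomLocationProbe actors tagged with type and row name, and stops after the first contiguous matching block.
; Removal destroys matching probes through a delayed loop; both operations display a loading screen widget.
; Unconnected leftovers include spawn-all and neighbour debug-line logic.
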(event `self.ReceiveBeginPlay`)

(event `SpawnSpecificActor`
  (params (ChosenPointType :type String))
  (bind _returnvalue (`GeoReferencingSystem.GetGeoReferencingSystem`))
  (bind _data_table (`self.Data Table`))
  (set `self.NotCompleted` (`self.NotCompleted`))
  (bind _outrownames (`DataTableFunctionLibrary.GetDataTableRowNames` _data_table))
  (bind _returnvalue_2 (`|CreateWidget` "/Game/DataProbeBP/LoadingScreen_Widget.LoadingScreen_Widget_C"))
  (`UserWidget.AddToViewport` _returnvalue_2 0)
  (for (_array_element _array_index) _outrownames
    (bind _returnvalue_3 (`|GetDataTableRow` _data_table _array_element)
      (:`then`
        (bind (_long _lat _type _distance _point_type) (break `/Game/DataProbeBP/ProbeDataStruct` _returnvalue_3))
        (if (== ChosenPointType _point_type)
          (set `self.Added` true)
          (bind _projectedcoordinates (`GeoReferencingSystem.GeographicToProjected` _returnvalue (`GeographicCoordinatesFunctionLibrary.MakeGeographicCoordinatesApproximation` _lat _long (`self.In Altitude`))))
          (bind _enginecoordinates (`GeoReferencingSystem.ProjectedToEngine` _returnvalue _projectedcoordinates))
          (bind _returnvalue_4 (`|SpawnActorFromClass` "/Game/DataProbeBP/BP_CustomLocationProbe.BP_CustomLocationProbe_C" (`KismetMathLibrary.Conv_VectorToTransform` _enginecoordinates) "Undefined" "OverrideRootScale" null null null))
          (`self.SetActorScale3D` _returnvalue_4 (10.0 10.0 1000.0))
          (set `/Game/DataProbeBP/BP_CustomLocationProbe.Type` _point_type _returnvalue_4)
          (set `self.actorLengths` (+ (`self.actorLengths`) 1))
          (set `/Game/DataProbeBP/BP_CustomLocationProbe.DataRowName` (`KismetStringLibrary.Conv_StringToName` (`KismetStringLibrary.Conv_IntToString` (+ _array_index 2))) _returnvalue_4)
          (elif (`self.Added`)
            (set `self.Added` false)
            (break))))))
  (`Widget.RemoveFromParent` _returnvalue_2))

(event `DestorySpecficActor`
  (params (ChosenDeletedPointType :type String))
  (bind _returnvalue (`|CreateWidget` "/Game/DataProbeBP/LoadingScreen_Widget.LoadingScreen_Widget_C"))
  (`UserWidget.AddToViewport` _returnvalue 0)
  (bind _outactors (`GameplayStatics.GetAllActorsOfClass` "/Game/DataProbeBP/BP_CustomLocationProbe.BP_CustomLocationProbe_C"))
  (bind _array_element (`/Game/DataProbeBP/MyMacroLibary.ForLoopWithDelay` _outactors)
    (:`Loop Body`
      (if (== ChosenDeletedPointType (`/Game/DataProbeBP/BP_CustomLocationProbe.Type` _array_element))
        (`self.K2_DestroyActor` _array_element)))
    (:`Completed`
      (`Widget.RemoveFromParent` _returnvalue))))

(fn `UserConstructionScript`)